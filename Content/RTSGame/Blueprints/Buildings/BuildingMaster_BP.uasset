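; BuildingMaster_BP is a building base for an RTS, with a configurable mesh, entrance, collision box and employee list.
; On BeginPlay it creates its own Building_HUD widget and binds to the camera controller's HUD request event.
; When a request targets this building, a timeline macro glides the camera pawn toward it while the HUD appears, input switches to UI-only, and camera navigation and main HUD are disabled.
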(event `self.ReceiveBeginPlay`
  ;[1 1 1] Begin Play
  (bind _ascamera_pawn_controller (cast `/Game/RTSGame/Blueprints/CameraPawnController` (`GameplayStatics.GetPlayerController` 0)))
  (bind _output_get (set `self.ControllerRef` _ascamera_pawn_controller))
  (add `/Game/RTSGame/Blueprints/CameraPawnController.HUDRequest` _output_get (`|CreateDelegate` :!event `DisplayHUD`))
  (bind _returnvalue (`|CreateWidget` "/Game/RTSGame/HUDs/Building_HUD.Building_HUD_C" null self (`self.ControllerRef`)))
  (set `self.BuildingHUD` _returnvalue))

(event `DisplayHUD`
  (params (Actor :type "Actor Object Reference"))
  (bind _controllerref (`self.ControllerRef`))
  ;[1 1 1] Display HUD
  (if (== Actor self)
    (`|ExecutionSequence`
      (:`then_0`
        (bind (_direction _speed) (`Timeline|LerpLocationTimeline` :!via `PlayFromStart`)
          (:`Update`
            (`self.K2_SetActorLocation` (`/Game/RTSGame/Blueprints/CameraPawnController.CameraPawnRef` (`self.ControllerRef`)) (`/Game/RTSGame/Libraries/FunctionLibrary.HUD_LerpLocation` (`self.K2_GetActorLocation` (`/Game/RTSGame/Blueprints/CameraPawnController.CameraPawnRef` (`self.ControllerRef`))) (`self.K2_GetActorLocation`) _speed) false false))))
      (:`then_1`
        (`UserWidget.AddToViewport` (`self.BuildingHUD`) 0)
        (`WidgetBlueprintLibrary.SetInputMode_UIOnlyEx` _controllerref null "LockAlways")
        (set `/Game/RTSGame/Blueprints/CameraPawnController.DisableCamNav` true _controllerref)
        (`Widget.SetIsEnabled` (`/Game/RTSGame/Blueprints/CameraPawnController.MainHUDRef` _controllerref) false)))))

(fn `GetEmployees`
  (returns (HasEmployees :type Boolean) (NumberOfEmployees :type Integer) (ListOfEmployees :type "Array of /Game/RTSGame/Blueprints/AI/NPC_BP Object Reference"))
  (bind _employees (`self.Employees`))
  (bind _returnvalue (`KismetArrayLibrary.Array_Length` _employees))
  (return (> _returnvalue 0) _returnvalue _employees))

(fn `UserConstructionScript`
  (`StaticMeshComponent.SetStaticMesh` (`self.StaticMesh`) (`self.DisplayMesh`))
  (`/Game/RTSGame/Libraries/FunctionLibrary.SetBuildingEntrance` (`self.Entrance`) (`self.StaticMesh`))
  (`/Game/RTSGame/Libraries/FunctionLibrary.SetBuildingCollisionBox` (`self.Collision`) (`self.StaticMesh`)))