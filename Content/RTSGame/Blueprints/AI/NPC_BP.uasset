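; NPC character for an RTS game, given a random sex, matching body colour and enum-drawn name at construction.
; Walk speed is base speed divided by the game state's speed multiplier, refreshed on game-speed updates.
; A HUD request opens its widget in UI-only input, lerps the camera pawn over, then a Tick gate keeps the camera following the NPC in X/Y.
; SetIsBusy writes a busy flag to the AI blackboard.
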(event `self.ReceiveBeginPlay`
  ;[1 1 1] Begin Play
  (bind _asnpc_aicontroller (cast `/Game/RTSGame/Blueprints/AI/NPC_AIController` (`AIBlueprintHelperLibrary.GetAIController` self)))
  (set `self.AIControllerRef` _asnpc_aicontroller)
  (bind _ascamera_pawn_controller (cast `/Game/RTSGame/Blueprints/CameraPawnController` (`GameplayStatics.GetPlayerController` 0)))
  (bind _output_get (set `self.CameraControllerRef` _ascamera_pawn_controller))
  (add `/Game/RTSGame/Blueprints/CameraPawnController.HUDRequest` _output_get (`|CreateDelegate` :!event `DisplayHUD`))
  (bind _returnvalue (`|CreateWidget` "/Game/RTSGame/HUDs/NPC_HUD.NPC_HUD_C" null self))
  (set `self.NPC_HUD` _returnvalue)
  (add `/Game/RTSGame/GameBP/MyGameState.UpdateGameSpeed` (`self.GameStateRef`) (`|CreateDelegate` :!event `UpdateWalkSpeed`))
  (`self.UpdateWalkSpeed` 0.0))

(event `UpdateWalkSpeed`
  (params (TimeUnit :type "Float (double-precision)"))
  ;[1 1 1] Update Walk Speed
  (set `CharacterMovementComponent.MaxWalkSpeed` (/ (`self.BaseWalkSpeed`) (`/Game/RTSGame/GameBP/MyGameState.SpeedMultiplier` (`self.GameStateRef`))) (`self.CharacterMovement`)))

(event `DisplayHUD`
  (params (Actor :type "Actor Object Reference"))
  (bind _cameracontrollerref (`self.CameraControllerRef`))
  ;[1 1 1] Display HUD
  (if (and (== Actor self) (not (`self.bHidden`)))
    (`UserWidget.AddToViewport` (`self.NPC_HUD`) 0)
    (`WidgetBlueprintLibrary.SetInputMode_UIOnlyEx` _cameracontrollerref null "LockAlways")
    (`Widget.SetIsEnabled` (`/Game/RTSGame/Blueprints/CameraPawnController.MainHUDRef` _cameracontrollerref) false)
    (bind (_direction _speed) (`Timeline|LerpLocationTimeline` :!via `PlayFromStart`)
      (:`Update`
        (`self.K2_SetActorLocation` (`/Game/RTSGame/Blueprints/CameraPawnController.CameraPawnRef` (`self.CameraControllerRef`)) (`/Game/RTSGame/Libraries/FunctionLibrary.HUD_LerpLocation` (`self.K2_GetActorLocation` (`/Game/RTSGame/Blueprints/CameraPawnController.CameraPawnRef` (`self.CameraControllerRef`))) (`self.K2_GetActorLocation`) _speed) false false))
      (:`Finished`
        (set `/Game/RTSGame/Blueprints/CameraPawnController.DisableCamNav` true (`self.CameraControllerRef`))
        (`self.OpenFollowGate`)))))

(event `self.ReceiveTick`
  (params (DeltaSeconds :type "Float (single-precision)"))
  (bind (_returnvalue_x _returnvalue_y) (`KismetMathLibrary.BreakVector` (`self.K2_GetActorLocation`)))
  (bind _camerapawnref (`/Game/RTSGame/Blueprints/CameraPawnController.CameraPawnRef` (`self.CameraControllerRef`)))
  (bind (_returnvalue_x_2 _returnvalue_y_2 _returnvalue_z) (`KismetMathLibrary.BreakVector` (`self.K2_GetActorLocation` _camerapawnref)))
  ;[1 1 1] Tick
  (`/Engine/EditorBlueprintResources/StandardMacros.Gate` true :!label _label
    (:`Exit`
      (`self.K2_SetActorLocation` _camerapawnref (`KismetMathLibrary.MakeVector` _returnvalue_x _returnvalue_y _returnvalue_z) false false))))

(event `OpenFollowGate`
  ;[1 1 1] Tick
  (goto _label :!via `Open`))

(event `CloseFollowGate`
  ;[1 1 1] Tick
  (goto _label :!via `Close`))

(fn `GetRandomName`
  (params (Sex :type "/Game/RTSGame/Enums/NPCSexType_ENUM Enum"))
  (returns (Name :type String))
  (if (`|EnumEquality` Sex "NewEnumerator0")
    (return (`|GetEnumeratorNameAsString` (enumliteral `/Game/RTSGame/Enums/NPCNameMale_ENUM` (cast `/Game/RTSGame/Enums/NPCNameMale_ENUM` (`KismetMathLibrary.Conv_IntToByte` (`KismetMathLibrary.RandomIntegerInRange` 0 (- (enumcount `/Game/RTSGame/Enums/NPCNameMale_ENUM`) 1)))))))
    (else
      (return (`|GetEnumeratorNameAsString` (enumliteral `/Game/RTSGame/Enums/NPCNameFemale_ENUM` (cast `/Game/RTSGame/Enums/NPCNameFemale_ENUM` (`KismetMathLibrary.Conv_IntToByte` (`KismetMathLibrary.RandomIntegerInRange` 0 (- (enumcount `/Game/RTSGame/Enums/NPCNameFemale_ENUM`) 1))))))))))

(fn `RandomNPCFeatures`
  (locals (MaterialInstance :type "MaterialInstanceDynamic Object Reference") (FemaleColor :type "LinearColor Structure" :default (struct :`R` 0.451 :`G` 0.028 :`B` 0.266)) (MaleColor :type "LinearColor Structure" :default (struct :`R` 0.061 :`G` 0.107 :`B` 0.451)))
  (bind _materialinstance (`local.MaterialInstance`))
  (bind _returnvalue (`PrimitiveComponent.CreateDynamicMaterialInstance` (`self.Mesh`) 0 "/Game/RTSGame/Character/Materials/M_UE4Man_Body_Inst.M_UE4Man_Body_Inst"))
  (set `local.MaterialInstance` _returnvalue)
  (if (`|EnumEquality` (enumliteral `/Game/RTSGame/Enums/NPCSexType_ENUM` (cast `/Game/RTSGame/Enums/NPCSexType_ENUM` (`KismetMathLibrary.Conv_IntToByte` (`KismetMathLibrary.RandomIntegerInRange` 0 1)))) "NewEnumerator0")
    (`MaterialInstanceDynamic.SetVectorParameterValue` _materialinstance "BodyColor" (`local.MaleColor`))
    (bind _name (`self.GetRandomName` "NewEnumerator0"))
    (set `self.MyProfile` (make `/Game/RTSGame/Structs/NPCProfile_Struct` _name))
    (else
      (`MaterialInstanceDynamic.SetVectorParameterValue` _materialinstance "BodyColor" (`local.FemaleColor`))
      (bind _name_2 (`self.GetRandomName` "NewEnumerator1"))
      (set `self.MyProfile` (make `/Game/RTSGame/Structs/NPCProfile_Struct` _name_2 "NewEnumerator1")))))

(fn `SetIsBusy`
  (params (IsBusy :type Boolean))
  (`BlackboardComponent.SetValueAsBool` (`AIBlueprintHelperLibrary.GetBlackboard` (`self.AIControllerRef`)) (`self.IsBusy`) IsBusy)
  (return))

(fn `UserConstructionScript`
  (`self.RandomNPCFeatures`))