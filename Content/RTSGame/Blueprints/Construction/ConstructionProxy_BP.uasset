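; Construction proxy actor for the RTS that stands in as a ghost-material building until its construction time has elapsed.
; Tick advances a clock scaled by game-speed time unit and active worker count, pausing without workers.
; On completion it signals construction completed, releases and unhides workers, then destroys itself.
; A controller HUD request glides the camera to the proxy and opens its widget, disabling navigation and main HUD.
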(event `self.ReceiveBeginPlay`
  ;[1 1 1] Begin Play
  (bind _output_get (set `self.GameStateRef` (cast `/Game/RTSGame/GameBP/MyGameState` (`GameplayStatics.GetGameState`) :!pure true)))
  (add `/Game/RTSGame/GameBP/MyGameState.UpdateGameSpeed` _output_get (`|CreateDelegate` :!event `AdjustTime`))
  (bind _timeunit (`/Game/RTSGame/GameBP/MyGameState.GetCurrentTimeUnit` (`self.GameStateRef`)))
  (set `self.TimeUnit` _timeunit)
  (bind _ascamera_pawn_controller (cast `/Game/RTSGame/Blueprints/CameraPawnController` (`GameplayStatics.GetPlayerController` 0)))
  (bind _output_get_2 (set `self.ControllerRef` _ascamera_pawn_controller))
  (add `/Game/RTSGame/Blueprints/CameraPawnController.HUDRequest` _output_get_2 (`|CreateDelegate` :!event `DisplayHUD`))
  (bind _returnvalue (`|CreateWidget` "/Game/RTSGame/HUDs/Proxy_HUD.Proxy_HUD_C" null self (`self.ControllerRef`)))
  (set `self.ProxyHUD` _returnvalue))

(event `self.ReceiveTick`
  (params (DeltaSeconds :type "Float (single-precision)"))
  ;[1 1 1] Tick
  (set `self.Delta` DeltaSeconds)
  (if (not (`self.IsConstructionComplete`))
    (`self.DoWork`)
    (if (>= (`self.WorkTimeSpent`) (`self.ConstructionTime`))
      (set `self.IsConstructionComplete` true)
      (`self.ConstructionCompleted` self)
      (`self.WorkComplete`)
      (if (`Widget.IsInViewport` (`self.ProxyHUD`))
        (`/Game/RTSGame/HUDs/Proxy_HUD.Remove HUD` (`self.ProxyHUD`)))
      (`KismetSystemLibrary.Delay` 0.2)
      (`self.K2_DestroyActor`))))

(event `AdjustTime`
  (params (TimeUnit :type "Float (double-precision)"))
  ;[1 1 1] Adjust Time
  (set `self.TimeUnit` TimeUnit))

(event `DisplayHUD`
  (params (Actor :type "Actor Object Reference"))
  (bind _controllerref (`self.ControllerRef`))
  ;[1 1 1] Display HUD
  (if (== Actor self)
    (`|ExecutionSequence`
      (:`then_0`
        (bind (_direction _speed) (`Timeline|Timeline_0` :!via `PlayFromStart`)
          (:`Update`
            (`self.K2_SetActorLocation` (`/Game/RTSGame/Blueprints/CameraPawnController.CameraPawnRef` (`self.ControllerRef`)) (`/Game/RTSGame/Libraries/FunctionLibrary.HUD_LerpLocation` (`self.K2_GetActorLocation` (`/Game/RTSGame/Blueprints/CameraPawnController.CameraPawnRef` (`self.ControllerRef`))) (`self.K2_GetActorLocation`) _speed) false false))))
      (:`then_1`
        (`UserWidget.AddToViewport` (`self.ProxyHUD`) 0)
        (`WidgetBlueprintLibrary.SetInputMode_UIOnlyEx` _controllerref null "LockAlways")
        (set `/Game/RTSGame/Blueprints/CameraPawnController.DisableCamNav` true _controllerref)
        (`Widget.SetIsEnabled` (`/Game/RTSGame/Blueprints/CameraPawnController.MainHUDRef` _controllerref) false)))))

(fn `DoWork`
  (bind _activeworkers (`self.GetWorkforce`))
  (if (> _activeworkers 0.0)
    (bind _output_get (set `self.Clockwork` (`/Game/RTSGame/Libraries/FunctionLibrary.SetClockwork` (`self.Delta`) (/ (`self.TimeUnit`) _activeworkers) (`self.Clockwork`))))
    (set `self.WorkTimeSpent` (* _output_get 60.0))
    (return)
    (else
      (return))))

(fn `GetWorkforce`
  (returns (ActiveWorkers :type "Float (double-precision)"))
  (return (`KismetMathLibrary.Conv_IntToDouble` (`KismetArrayLibrary.Array_Length` (`self.ActiveWorkers`)))))

(fn `ReportToShift`
  (params (Worker :type "/Game/RTSGame/Blueprints/AI/NPC_BP Object Reference"))
  (`KismetArrayLibrary.Array_Add` (`self.ActiveWorkers`) Worker)
  (return))

(fn `SetContructionTime`
  (params (WorkHours :type "Float (double-precision)"))
  (set `self.ConstructionTime` (* WorkHours 60.0))
  (return))

(fn `UserConstructionScript`
  (bind _staticmesh (`self.StaticMesh`))
  (`StaticMeshComponent.SetStaticMesh` _staticmesh (`self.DisplayMesh`))
  (`PrimitiveComponent.SetMaterial` _staticmesh 0 "/Game/RTSGame/Materials/GhostBuild_M_Inst.GhostBuild_M_Inst")
  (`/Game/RTSGame/Libraries/FunctionLibrary.SetBuildingEntrance` (`self.Entrance`) (`self.StaticMesh`))
  (`/Game/RTSGame/Libraries/FunctionLibrary.SetBuildingCollisionBox` (`self.Collision`) (`self.StaticMesh`)))

(fn `WorkComplete`
  (if (> (`self.GetWorkforce`) 0.0)
    (for _array_element (`self.ActiveWorkers`)
      (`/Game/RTSGame/Blueprints/AI/NPC_BP.SetIsBusy` _array_element false)
      (`self.SetActorHiddenInGame` _array_element false))
    (set `self.ActiveWorkers` (`|MakeArray` null :!type "/Game/RTSGame/Blueprints/AI/NPC_BP Object Reference"))
    (return)
    (else
      (return))))