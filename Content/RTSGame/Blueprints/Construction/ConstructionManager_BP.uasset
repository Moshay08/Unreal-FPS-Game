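; Construction manager for an RTS that queues building jobs and swaps finished construction proxies for real buildings.
; Each queued job spawns a proxy with its mesh and work hours, tracked in parallel arrays until completion triggers the swap.
; New proxies go to the nearest construction office with employees and no active job, or into a bid list when none is available.
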(event `BindConstructionComplete`
  (params (Proxy :type "/Game/RTSGame/Blueprints/Construction/ConstructionProxy_BP Object Reference"))
  (add `/Game/RTSGame/Blueprints/Construction/ConstructionProxy_BP.ConstructionCompleted` Proxy (`|CreateDelegate` :!event `ConstructionCompleted`)))

(event `ConstructionCompleted`
  (params (Proxy :type "/Game/RTSGame/Blueprints/Construction/ConstructionProxy_BP Object Reference"))
  (`self.FinishedConstruction` Proxy))

(fn `FinishedConstruction`
  (params (Proxy :type "/Game/RTSGame/Blueprints/Construction/ConstructionProxy_BP Object Reference"))
  (locals (Index :type Integer :default 0) (Config :type "/Game/RTSGame/Structs/Construction_Struct Structure"))
  (bind _proxies (`self.Proxies`))
  (bind _queue (`self.Queue`))
  (bind _index (`local.Index`))
  (bind (_buildingclass _proxyclass _transform) (break `/Game/RTSGame/Structs/Construction_Struct` (`local.Config`)))
  (bind _output_get (set `local.Index` (`KismetArrayLibrary.Array_Find` _proxies Proxy)))
  (set `local.Config` (`|GetArrayItem` _queue _output_get))
  (`KismetArrayLibrary.Array_Remove` _queue _index)
  (`KismetArrayLibrary.Array_Remove` _proxies _index)
  (`|SpawnActorFromClass` _buildingclass _transform "Undefined" "OverrideRootScale")
  (`self.K2_DestroyActor` Proxy))

(fn `InitialContractorSearch`
  (params (Proxy :type "/Game/RTSGame/Blueprints/Construction/ConstructionProxy_BP Object Reference"))
  (locals (Proxy_LOCAL :type "/Game/RTSGame/Blueprints/Construction/ConstructionProxy_BP Object Reference") (AllConstructionOffices_LOCAL :type "Array of /Game/RTSGame/Blueprints/Buildings/Commercial/ConstructionOffice_BP Object Reference") (SelectedOffice_LOCAL :type "/Game/RTSGame/Blueprints/Buildings/Commercial/ConstructionOffice_BP Object Reference") (DistanceToSite_LOCAL :type "Array of Float (double-precision)") (AvailableConstructionOffices_LOCAL :type "Array of /Game/RTSGame/Blueprints/Buildings/Commercial/ConstructionOffice_BP Object Reference"))
  (bind _proxy_local (`local.Proxy_LOCAL`))
  (set `local.Proxy_LOCAL` Proxy)
  (bind _outactors (`GameplayStatics.GetAllActorsOfClass` "/Game/RTSGame/Blueprints/Buildings/Commercial/ConstructionOffice_BP.ConstructionOffice_BP_C"))
  (bind _output_get (set `local.AllConstructionOffices_LOCAL` _outactors))
  (if (> (`KismetArrayLibrary.Array_Length` _output_get) 0)
    (for _array_element (`local.AllConstructionOffices_LOCAL`)
      (bind _output_get_2 (set `local.SelectedOffice_LOCAL` _array_element))
      (if (and (`/Game/RTSGame/Blueprints/Buildings/BuildingMaster_BP.GetEmployees` _output_get_2) (not (`/Game/RTSGame/Blueprints/Buildings/Commercial/ConstructionOffice_BP.GetJobStatus` _output_get_2)))
        (`KismetArrayLibrary.Array_Add` (`local.DistanceToSite_LOCAL`) (`self.GetDistanceTo` (`local.SelectedOffice_LOCAL`) (`local.Proxy_LOCAL`)))
        (`KismetArrayLibrary.Array_AddUnique` (`local.AvailableConstructionOffices_LOCAL`) (`local.SelectedOffice_LOCAL`))))
    (if (> (`KismetArrayLibrary.Array_Length` (`local.AvailableConstructionOffices_LOCAL`)) 0)
      (bind _output_get_3 (set `/Game/RTSGame/Blueprints/Construction/ConstructionProxy_BP.Contractor` (`|GetArrayItem` (`local.AvailableConstructionOffices_LOCAL`) (`KismetMathLibrary.MinOfFloatArray` (`local.DistanceToSite_LOCAL`))) _proxy_local))
      (`/Game/RTSGame/Blueprints/Buildings/Commercial/ConstructionOffice_BP.SetCurrentJob` _output_get_3 _proxy_local)
      (return)
      (else
        (`KismetArrayLibrary.Array_AddUnique` (`self.ConstructionBids`) (`local.Proxy_LOCAL`))
        (return)))
    (else
      (`KismetArrayLibrary.Array_AddUnique` (`self.ConstructionBids`) (`local.Proxy_LOCAL`))
      (return))))

(fn `QueueConstruction`
  (params (ConstructionStruct :type "/Game/RTSGame/Structs/Construction_Struct Structure"))
  (bind (_buildingclass _proxyclass _transform _displaymesh _workhoursrequired) (break `/Game/RTSGame/Structs/Construction_Struct` ConstructionStruct))
  (bind _returnvalue (`|SpawnActorFromClass` _proxyclass _transform "AlwaysSpawn" "OverrideRootScale" null _displaymesh))
  (`self.BindConstructionComplete` _returnvalue)
  (`KismetArrayLibrary.Array_Add` (`self.Proxies`) _returnvalue)
  (`KismetArrayLibrary.Array_Add` (`self.Queue`) ConstructionStruct)
  (`/Game/RTSGame/Blueprints/Construction/ConstructionProxy_BP.SetContructionTime` _returnvalue _workhoursrequired)
  (`self.InitialContractorSearch` _returnvalue))

(fn `UserConstructionScript`)